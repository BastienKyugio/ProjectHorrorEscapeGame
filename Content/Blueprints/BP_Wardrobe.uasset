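; BP_Wardrobe is an interactable wardrobe that opens and closes when used.
; Its Interact event checks the IsOpen flag, rotates two scene components in opposite directions to open or resets both to zero to close, then updates the flag.
; Rotations are set instantly, with no timeline or interpolation.
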(event EventBeginPlay)

(event Collision|EventActorBeginOverlap
  (params (OtherActor :type Actor%20Object%20Reference)))

(event EventTick
  (params (DeltaSeconds :type Float%20%28single-precision%29)))

(event EventInteract
  (params (Interactor :type Actor%20Object%20Reference))
  (if (Variables|Default|GetbIsOpen)
    (Transformation|SetRelativeRotation (Variables|Default|GetScene2) "0.000000,0.000000,0.000000" false false)
    (Transformation|SetRelativeRotation (Variables|Default|GetScene1) "0.000000,0.000000,0.000000" false false)
    (Variables|Default|SetbIsOpen false)
    (else
      (Transformation|SetRelativeRotation (Variables|Default|GetScene2) "0.000000,-120.000000,0.000000" false false)
      (Transformation|SetRelativeRotation (Variables|Default|GetScene1) "0.000000,120.000000,0.000000" false false)
      (Variables|Default|SetbIsOpen true))))

(fn ConstructionScript)