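; BPC_Inventory is an actor component that holds the player's inventory items and tracks which one is selected.
; TryAddItem always appends and returns true, while SelectItem marks an item as selected only if the inventory contains it, printing its ID for debugging.
; UseSelectedItem handles only the HealingItem ID, calling HealPlayer on the owning BP_FirstPersonCharacter, then removing the item and clearing the selection.
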(event EventBeginPlay)

(event EventTick
  (params (DeltaSeconds :type Float%20%28single-precision%29)))

(fn TryAddItem
  (params (ItemToAdd :type ST%20Item%20Data%20Structure))
  (Utilities|Array|Add (Variables|Default|GetInventoryItems) ItemToAdd)
  (return true))

(fn SelectItem
  (params (ItemToSelect :type ST%20Item%20Data%20Structure))
  (bind _output_get (LocalVariables|SetItem ItemToSelect))
  (if (Utilities|Array|ContainsItem (Variables|Default|GetInventoryItems) _output_get)
    (bind _output_get_2 (Variables|Default|SetSelectedItem (LocalVariables|GetItem)))
    (Development|PrintString (Utilities|String|ToString(Name) (.ItemId (Utilities|Struct|BreakST_ItemData _output_get_2))))
    (Variables|Default|SetbHasSelectedItem true)))

(fn UseSelectedItem
  (bind _inventoryitems (Variables|Default|GetInventoryItems))
  (if (Variables|Default|GetbHasSelectedItem)
    (if (== (.ItemId (Utilities|Struct|BreakST_ItemData (Variables|Default|GetSelectedItem))) "HealingItem")
      (bind _asbp_first_person_character (Utilities|Casting|CastToBP_FirstPersonCharacter (Components|GetOwner))
        (:then
          (Default|HealPlayer _asbp_first_person_character)
          (Utilities|Array|RemoveIndex _inventoryitems (Utilities|Array|FindItem _inventoryitems (Variables|Default|GetSelectedItem)))
          (Variables|Default|SetbHasSelectedItem false)
          (Variables|Default|SetSelectedItem "")
          (return true))
        (:CastFailed
          _))))
  (return false))