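; Base item actor that can be picked up through an Interact event.
; When pickup is allowed, it builds item data from its ID, name and description and tries to add it to the interactor's inventory component.
; A successful add destroys the actor, first starting the game mode's level timer if the item is the Screwdriver, matched by a hardcoded name check.
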(event EventBeginPlay)

(event Collision|EventActorBeginOverlap
  (params (OtherActor :type Actor%20Object%20Reference)))

(event EventTick
  (params (DeltaSeconds :type Float%20%28single-precision%29)))

(event EventInteract
  (params (Interactor :type Actor%20Object%20Reference))
  (bind _itemname (Variables|Default|GetItemName))
  (bind _returnvalue (Utilities|String|ToString(Text) _itemname))
  (if (Variables|Default|GetbCanPickUp)
    (bind _itemdata (CallFunction|GetItemData))
    (bind _success (Default|TryAddItem (Actor|GetComponentbyClass Interactor "/Game/Blueprints/BlueprintComposant/BPC_Inventory.BPC_Inventory_C") _itemdata))
    (if _success
      (Development|PrintString _returnvalue true true "(R=0.151789,G=1.000000,B=0.133354,A=1.000000)")
      (if (Utilities|Enum|Equal(Enum) _returnvalue "Screwdriver")
        (bind _asbp_first_person_game_mode (Utilities|Casting|CastToBP_FirstPersonGameMode (Game|GetGameMode)))
        (Default|StartLevelTimer _asbp_first_person_game_mode))
      (Actor|DestroyActor)
      (else
        (Development|PrintString "PickupFailed" true true "(R=1.000000,G=0.257189,B=0.218975,A=1.000000)")))))

(fn ConstructionScript)

(fn GetItemData
  (return (Utilities|Struct|MakeST_ItemData (Variables|Default|GetItemId) (Variables|Default|GetItemName) (Variables|Default|GetItemDescription))))