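; BP_ElectricityPannel is an interactable electrical panel with cables that the player can cut using a required inventory item.
; The first interaction opens the door by setting its relative rotation.
; Later interactions compare the first-person character's selected inventory item to RequiredItem, then swap both cables to cut meshes and a cut material.
; A wrong item only prints a debug hint to use a scalpel.
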(event EventBeginPlay)

(event Collision|EventActorBeginOverlap
  (params (OtherActor :type Actor%20Object%20Reference)))

(event EventTick
  (params (DeltaSeconds :type Float%20%28single-precision%29)))

(event EventInteract
  (params (Interactor :type Actor%20Object%20Reference))
  (bind _leftcable (Variables|Default|GetLeftCable))
  (bind _asbp_first_person_character (Utilities|Casting|CastToBP_FirstPersonCharacter Interactor))
  (if (Variables|Default|GetDoorIsOpen)
    (if (== (.ItemId (Utilities|Struct|BreakST_ItemData (Variables|/Game/Blueprints/BlueprintComposant/BPC_Inventory.BPC_Inventory_C|GetSelectedItem (Variables|/Game/FirstPerson/Blueprints/BP_FirstPersonCharacter.BP_FirstPersonCharacter_C|GetBPC_Inventory _asbp_first_person_character)))) (Variables|Default|GetRequiredItem))
      (Components|StaticMesh|SetStaticMesh _leftcable "/Game/Meshes/Geo_Cable_01_Cut.Geo_Cable_01_Cut")
      (Components|StaticMesh|SetStaticMesh (Variables|Default|GetRightCable) "/Game/Meshes/Geo_Cable_02_Cut.Geo_Cable_02_Cut")
      (Rendering|Material|SetMaterial _leftcable 0 "/Game/Material/MI_Electric_Panel_Cable_Cut.MI_Electric_Panel_Cable_Cut")
      (else
        (Development|PrintString "Use Scalpel")))
    (else
      (Variables|Default|SetDoorIsOpen true)
      (Transformation|SetRelativeRotation (Variables|Default|GetDoor) "0.000000,0.000000,0.000000" false false))))

(fn ConstructionScript)