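; BP_HealingItem is an interactable healing item, presented to the player as a Syringe.
; It overrides GetItemData to return an item data struct identifying it as HealingItem.
; Interact and the construction script only call the parent class, and the file defines no healing logic of its own.
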(event EventBeginPlay
  (|CallParentFunction) ; This node is disabled and will not be called.\nDrag off pins to build functionality.
)

(event Collision|EventActorBeginOverlap
  (params (OtherActor :type Actor%20Object%20Reference))
  (|CallParentFunction OtherActor) ; This node is disabled and will not be called.\nDrag off pins to build functionality.
)

(event EventTick
  (params (DeltaSeconds :type Float%20%28single-precision%29))
  (|CallParentFunction DeltaSeconds) ; This node is disabled and will not be called.\nDrag off pins to build functionality.
)

(event EventInteract
  (params (Interactor :type Actor%20Object%20Reference))
  (|CallParentFunction Interactor))

(fn ConstructionScript
  (|CallParentFunction))

(fn GetItemData
  (|CallParentFunction)
  (return (Utilities|Struct|MakeST_ItemData "HealingItem" "Syringe" "Heal injuries" 0 0 0 0 true)))