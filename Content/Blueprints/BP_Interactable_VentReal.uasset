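; Interactable vent that opens when the interactor's selected inventory item matches the required item ID, otherwise printing a wrong-item message.
; On success it works through four screw components in sequence, snapping the player's view toward each.
; A Retire timeline spins and shifts each screw along Z, then re-triggers RetireScrew for the next.
; After the last, it resets look input, marks itself open and destroys itself following a short delay.
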(event Custom|AnimRetire
  (Variables|Default|SetLockedScrew (Utilities|Array|Get(acopy) (Variables|Default|GetScrewsList) (Variables|Default|GetIndex))))

(event Custom|RetireScrew
  (bind _returnvalue (Game|GetPlayerController 0))
  (bind _lockedscrew (Variables|Default|GetLockedScrew))
  (bind _lockedscrew_2 (Variables|Default|GetLockedScrew))
  (bind _relativelocation (Variables|/Script/Engine.SceneComponent|GetRelativeLocation _lockedscrew_2))
  (bind _relativerotation (Variables|/Script/Engine.SceneComponent|GetRelativeRotation _lockedscrew))
  (CallFunction|AnimRetire)
  (Input|SetIgnoreLookInput _returnvalue false)
  (Pawn|SetControlRotation _returnvalue (Math|Rotator|FindLookatRotation (Camera|GetCameraLocation (Variables|/Script/Engine.PlayerController|GetPlayerCameraManager _returnvalue)) (Transformation|GetWorldLocation (Variables|Default|GetLockedScrew))))
  (bind _newtrack_0 (Timeline|Retire PlayFromStart)
    (:Update
      (Transformation|SetRelativeRotation (Variables|Default|GetLockedScrew) (Math|Rotator|Lerp(Rotator) (Variables|/Script/Engine.SceneComponent|GetRelativeRotation _lockedscrew) (Math|Rotator|MakeRotator (.roll _relativerotation) (.pitch _relativerotation) (+ (.yaw _relativerotation) 9e+01)) _newtrack_0) false false)
      (Transformation|SetRelativeLocation (Variables|Default|GetLockedScrew) (Math|Vector|MakeVector (.x _relativelocation) (.y _relativelocation) (Math|Float|Lerp (.z _relativelocation) 8.0 _newtrack_0)) false false))
    (:Finished
      (bind _result (Math|Integer|IncrementInt (Variables|Default|GetIndex))
        (:%20%20
          (if (< _result (Utilities|Array|Length (Variables|Default|GetScrewsList)))
            (CallFunction|RetireScrew)
            (else
              (Input|ResetIgnoreLookInput (Game|GetPlayerController 0))
              (Variables|Default|SetbIsOpen true)
              (Utilities|FlowControl|Delay 1.0)
              (Actor|DestroyActor))))))))

(event EventBeginPlay
  (|CallParentFunction)
  (Utilities|Array|Add (Variables|Default|GetScrewsList) (Variables|Default|GetScrew_1))
  (Utilities|Array|Add (Variables|Default|GetScrewsList) (Variables|Default|GetScrew_2))
  (Utilities|Array|Add (Variables|Default|GetScrewsList) (Variables|Default|GetScrew_3))
  (Utilities|Array|Add (Variables|Default|GetScrewsList) (Variables|Default|GetScrew_4)))

(event Collision|EventActorBeginOverlap
  (params (OtherActor :type Actor%20Object%20Reference))
  (|CallParentFunction OtherActor) ; This node is disabled and will not be called.\nDrag off pins to build functionality.
)

(event EventTick
  (params (DeltaSeconds :type Float%20%28single-precision%29))
  (|CallParentFunction DeltaSeconds) ; This node is disabled and will not be called.\nDrag off pins to build functionality.
)

(event EventInteract
  (params (Interactor :type Actor%20Object%20Reference))
  (if (not (Variables|Default|GetbIsOpen))
    (if (== (.ItemId (Utilities|Struct|BreakST_ItemData (Variables|/Game/Blueprints/BlueprintComposant/BPC_Inventory.BPC_Inventory_C|GetSelectedItem (Actor|GetComponentbyClass Interactor "/Game/Blueprints/BlueprintComposant/BPC_Inventory.BPC_Inventory_C")))) (Variables|Default|GetRequiredItemID))
      (Variables|Default|SetIndex 0)
      (CallFunction|RetireScrew)
      (Development|PrintString "Good Item ! " true true "(R=0.990367,G=1.000000,B=0.085471,A=1.000000)")
      (else
        (Development|PrintString "Wrong Item ! " true true "(R=0.990367,G=1.000000,B=0.085471,A=1.000000)")))))

(fn ConstructionScript
  (|CallParentFunction))