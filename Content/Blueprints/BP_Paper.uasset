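; BP_Paper is an interactable paper item that carries a four-digit number in its item data.
; It is a child Blueprint that leaves BeginPlay, Interact and construction to its parent.
; Its GetItemData override keeps the parent's ID, name and description and fills the four PaperDigit fields with hardcoded values.
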(event EventBeginPlay
  (|CallParentFunction))

(event Collision|EventActorBeginOverlap
  (params (OtherActor :type Actor%20Object%20Reference))
  (|CallParentFunction OtherActor) ; This node is disabled and will not be called.\nDrag off pins to build functionality.
)

(event EventTick
  (params (DeltaSeconds :type Float%20%28single-precision%29))
  (|CallParentFunction DeltaSeconds) ; This node is disabled and will not be called.\nDrag off pins to build functionality.
)

(event EventInteract
  (params (Interactor :type Actor%20Object%20Reference))
  (|CallParentFunction Interactor))

(fn ConstructionScript
  (|CallParentFunction))

(fn GetItemData
  (bind _itemdata (|CallParentFunction))
  (return (Utilities|Struct|MakeST_ItemData (.ItemId (Utilities|Struct|BreakST_ItemData _itemdata)) (.ItemName (Utilities|Struct|BreakST_ItemData _itemdata)) (.ItemDescription (Utilities|Struct|BreakST_ItemData _itemdata)) 3 7 2 5)))