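; Interactable vent actor that opens when the interactor has the required item selected.
; On Interact, a closed vent compares the selected item ID in the interactor's BPC_Inventory against RequiredItemID.
; A match calls OpenVent, which snaps the static mesh to a rotated open pose and sets IsOpen, so further interactions do nothing.
; Success and failure are reported only through debug PrintString messages.
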(event EventBeginPlay
  (|CallParentFunction) ; This node is disabled and will not be called.\nDrag off pins to build functionality.
)

(event Collision|EventActorBeginOverlap
  (params (OtherActor :type Actor%20Object%20Reference))
  (|CallParentFunction OtherActor) ; This node is disabled and will not be called.\nDrag off pins to build functionality.
)

(event EventTick
  (params (DeltaSeconds :type Float%20%28single-precision%29))
  (|CallParentFunction DeltaSeconds) ; This node is disabled and will not be called.\nDrag off pins to build functionality.
)

(event EventInteract
  (params (Interactor :type Actor%20Object%20Reference))
  (if (not (Variables|Default|GetbIsOpen))
    (if (== (.ItemId (Utilities|Struct|BreakST_ItemData (Variables|/Game/Blueprints/BlueprintComposant/BPC_Inventory.BPC_Inventory_C|GetSelectedItem (Actor|GetComponentbyClass Interactor "/Game/Blueprints/BlueprintComposant/BPC_Inventory.BPC_Inventory_C")))) (Variables|Default|GetRequiredItemID))
      (CallFunction|OpenVent)
      (Development|PrintString "Good Item ! " true true "(R=0.990367,G=1.000000,B=0.085471,A=1.000000)")
      (else
        (Development|PrintString "Wrong Item ! " true true "(R=0.990367,G=1.000000,B=0.085471,A=1.000000)")))))

(fn ConstructionScript
  (|CallParentFunction))

(fn OpenVent
  (Transformation|SetRelativeRotation (Variables|Default|GetStaticMesh) "90.000000,0.000000,0.000000" false false)
  (Variables|Default|SetbIsOpen true)
  (Development|PrintString "Hello"))