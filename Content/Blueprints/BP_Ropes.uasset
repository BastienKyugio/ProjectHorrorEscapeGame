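; Interactable ropes that bind the first-person player until cut free with a Needle.
; On Interact, it reads the selected item from the interactor's BPC_Inventory component and prints a hint unless that item is the Needle.
; With the Needle, it enables the character's movement, flags it freed, swaps its first-person mesh to SKM_Manny_Simple, and destroys both the ropes and the FakeBody actor.
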(event EventBeginPlay)

(event Collision|EventActorBeginOverlap
  (params (OtherActor :type Actor%20Object%20Reference)))

(event EventTick
  (params (DeltaSeconds :type Float%20%28single-precision%29)))

(event EventInteract
  (params (Interactor :type Actor%20Object%20Reference))
  (bind _output_get (Variables|Default|SetInteractor Interactor))
  (bind _output_get_2 (Variables|Default|SetInventory (Actor|GetComponentbyClass _output_get "/Game/Blueprints/BlueprintComposant/BPC_Inventory.BPC_Inventory_C")))
  (if (Variables|/Game/Blueprints/BlueprintComposant/BPC_Inventory.BPC_Inventory_C|GetbHasSelectedItem _output_get_2)
    (if (== (.ItemId (Utilities|Struct|BreakST_ItemData (Variables|/Game/Blueprints/BlueprintComposant/BPC_Inventory.BPC_Inventory_C|GetSelectedItem (Variables|Default|GetInventory)))) "Needle")
      (bind _asbp_first_person_character (Utilities|Casting|CastToBP_FirstPersonCharacter (Variables|Default|GetInteractor)))
      (Variables|/Game/FirstPerson/Blueprints/BP_FirstPersonCharacter.BP_FirstPersonCharacter_C|SetbCanMove _asbp_first_person_character true)
      (Variables|/Game/FirstPerson/Blueprints/BP_FirstPersonCharacter.BP_FirstPersonCharacter_C|SetbIsFreed _asbp_first_person_character true)
      (Components|SkeletalMesh|SetSkeletalMeshAsset (Variables|/Game/FirstPerson/Blueprints/BP_FirstPersonCharacter.BP_FirstPersonCharacter_C|GetFirstPersonMesh _asbp_first_person_character) "/Game/Characters/Mannequins/Meshes/SKM_Manny_Simple.SKM_Manny_Simple")
      (Actor|DestroyActor)
      (Actor|DestroyActor (Variables|Default|GetFakeBody))
      (Development|PrintString "I'm free !" true true "(R=1.000000,G=0.968379,B=0.927889,A=1.000000)")
      (else
        (Development|PrintString "I need a needle" true true "(R=1.000000,G=0.968379,B=0.927889,A=1.000000)")))
    (else
      (Development|PrintString "I need a needle" true true "(R=1.000000,G=0.968379,B=0.927889,A=1.000000)"))))

(fn ConstructionScript)